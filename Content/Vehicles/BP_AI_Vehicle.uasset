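; AI-driven vehicle Blueprint that follows a spline path and caps its speed.
; Each tick it takes the first Path actor's spline, aims at a point 500 units ahead along the nearest tangent, and maps the yaw error to steering input.
; Throttle is full until speed in km/h exceeds MaxSpeed, then zero, with speed printed on screen.
; Stop and Resume functions toggle the handbrake.
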(event EventTick
  (params (DeltaSeconds :type Float%20%28single-precision%29))
  (CallFunction|SteerVehicle)
  (CallFunction|MaintainSpeed))

(fn ConstructionScript
  (|CallParentFunction))

(fn GetPath
  (params (Splines :type Array%20of%20Path%20Object%20References))
  (bind _returnvalue (Transformation|GetActorLocation))
  (bind _output (Utilities|Array|Get(acopy) Splines))
  (bind _spline (Variables|/Game/Vehicles/Path.Path_C|GetSpline _output))
  (return (Math|Float|MapRangeClamped (.yaw (Math|Rotator|Delta(Rotator) (Math|Rotator|FindLookatRotation _returnvalue (Spline|FindLocationClosesttoWorldLocation _spline (+ (* (Math|Vector|Normalize (Class|SplineComponent|FindTangentClosesttoWorldLocation _spline _returnvalue "World")) 5e+02) _returnvalue) "World")) (Transformation|GetActorRotation))) -9e+01 9e+01 -1.0 1.0)))

(fn SteerVehicle
  (bind _outactors (Actor|GetAllActorsOfClass "/Game/Vehicles/Path.Path_C"))
  (bind _steering (CallFunction|GetPath _outactors))
  (Class|ChaosVehicleMovementComponent|SetSteeringInput (Variables|Default|GetVehicleMovementComponent) _steering))

(fn MaintainSpeed
  (bind _returnvalue (Transformation|GetVelocity))
  (bind _vehiclemovementcomponent (Variables|Default|GetVehicleMovementComponent))
  (bind _returnvalue_2 (Math|Vector|VectorLength _returnvalue))
  (bind _returnvalue_3 (* _returnvalue_2 0.036))
  (Development|PrintString (Utilities|String|Append (Utilities|String|ToString(Float) _returnvalue_3) " kmph"))
  (if (> _returnvalue_3 (Variables|Default|GetMaxSpeed))
    (Class|ChaosVehicleMovementComponent|SetThrottleInput _vehiclemovementcomponent 0.0)
    (else
      (Class|ChaosVehicleMovementComponent|SetThrottleInput _vehiclemovementcomponent 1.0))))

(fn Stop
  (Class|ChaosVehicleMovementComponent|SetHandbrakeInput (Variables|Default|GetVehicleMovementComponent) true))

(fn Resume
  (Class|ChaosVehicleMovementComponent|SetHandbrakeInput (Variables|Default|GetVehicleMovementComponent) false))