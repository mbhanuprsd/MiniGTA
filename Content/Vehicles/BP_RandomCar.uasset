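; BP_RandomCar is a vehicle Blueprint that sets its car model from a data table at construction time.
; After the parent construction script runs, it looks up the VehicleTable row at VehicleIndex and applies that row's skeletal mesh and physics asset to Mesh.
; If that lookup fails, it tries a random row, then the hardcoded "v_1" row.
; The event graph holds no active logic.
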(event EventBeginPlay)

(event Collision|EventActorBeginOverlap
  (params (OtherActor :type Actor%20Object%20Reference)))

(event EventTick
  (params (DeltaSeconds :type Float%20%28single-precision%29)))

(fn ConstructionScript
  (bind _mesh (Variables|Character|GetMesh))
  (|CallParentFunction)
  (bind _outrownames (DataTable|GetDataTableRowNames "/Game/Vehicles/VehicleTable.VehicleTable"))
  (bind _returnvalue (Utilities|GetDataTableRow "/Game/Vehicles/VehicleTable.VehicleTable" (Utilities|Array|Get(acopy) _outrownames (Variables|Default|GetVehicleIndex)))
    (:then
      (Class|SkinnedMeshComponent|SetSkeletalMesh _mesh (.vehiclemesh _returnvalue) true)
      (Components|SkinnedMesh|SetPhysicsAsset _mesh (.vehiclephysics _returnvalue) true))
    (:RowNotFound
      (bind _returnvalue_2 (Utilities|GetDataTableRow "/Game/Vehicles/VehicleTable.VehicleTable" (Utilities|Array|Get(acopy) _outrownames (Math|Random|RandomInteger (Utilities|Array|Length _outrownames))))
        (:then
          (Class|SkinnedMeshComponent|SetSkeletalMesh _mesh (.vehiclemesh _returnvalue_2) true)
          (Components|SkinnedMesh|SetPhysicsAsset _mesh (.vehiclephysics _returnvalue_2) true))
        (:RowNotFound
          (bind _returnvalue_3 (Utilities|GetDataTableRow "/Game/Vehicles/VehicleTable.VehicleTable" "v_1")
            (:then
              (Class|SkinnedMeshComponent|SetSkeletalMesh _mesh (.vehiclemesh _returnvalue_3) true)
              (Components|SkinnedMesh|SetPhysicsAsset _mesh (.vehiclephysics _returnvalue_3) true))))))))