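; BP_ControllableVehicle is a player-drivable vehicle that maps input directly to its VehicleMovementComponent.
; Throttle, steering and brake axes pass straight through, while gear up and down presses set the change inputs to true with no release handling.
; The handbrake toggles on each press rather than being held.
; Interact calls RepossesFromVehicle on the stored Driver to hand control back from the vehicle.
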(event Input|ActionEvents|InputActionGearChangeUp
  (params (Key :type Key%20Structure :default "None"))
  (:Pressed
    (Class|ChaosVehicleMovementComponent|SetChangeUpInput (Variables|Default|GetVehicleMovementComponent) true)))

(event Input|ActionEvents|InputActionGearChangeDown
  (params (Key :type Key%20Structure :default "None"))
  (:Pressed
    (Class|ChaosVehicleMovementComponent|SetChangeDownInput (Variables|Default|GetVehicleMovementComponent) true)))

(event Input|ActionEvents|InputActionHandbrake
  (params (Key :type Key%20Structure :default "None"))
  (bind _vehiclemovementcomponent (Variables|Default|GetVehicleMovementComponent))
  (:Pressed
    (Class|ChaosVehicleMovementComponent|SetHandbrakeInput _vehiclemovementcomponent (not (Class|ChaosVehicleMovementComponent|GetHandbrakeInput _vehiclemovementcomponent)))))

(event Input|ActionEvents|InputActionInteract
  (params (Key :type Key%20Structure :default "None"))
  (:Pressed
    (Default|RepossesfromVehicle (Variables|Default|GetDriver))))

(event Input|AxisEvents|InputAxisThrottle
  (params (AxisValue :type Float%20%28single-precision%29))
  (Class|ChaosVehicleMovementComponent|SetThrottleInput (Variables|Default|GetVehicleMovementComponent) AxisValue))

(event Input|AxisEvents|InputAxisSteering
  (params (AxisValue :type Float%20%28single-precision%29))
  (Class|ChaosVehicleMovementComponent|SetSteeringInput (Variables|Default|GetVehicleMovementComponent) AxisValue))

(event Input|AxisEvents|InputAxisBrake
  (params (AxisValue :type Float%20%28single-precision%29))
  (Class|ChaosVehicleMovementComponent|SetBrakeInput (Variables|Default|GetVehicleMovementComponent) AxisValue))

(fn ConstructionScript
  (|CallParentFunction))