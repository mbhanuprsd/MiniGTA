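; Base pedestrian character the player walks, jumps and looks around with, able to get into and out of controllable vehicles.
; Interact box-traces ahead for a BP_ControllableVehicle, then disables collision, attaches the pedestrian to its Driver socket and passes possession to it.
; RepossesFromVehicle reverses this by detaching, restoring collision and repossessing the pedestrian.
; Movement reuses driving input names like Throttle, Steering and Handbrake, and SwitchCharacter picks a random skeletal mesh from a data table.
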(event EventBeginPlay
  (bind _outrownames (DataTable|GetDataTableRowNames "/Game/Pedestrians/CharacterTable.CharacterTable"))
  (Variables|Default|SetmeshCount (Utilities|Array|Length _outrownames)))

(event Input|ActionEvents|InputActionHandbrake
  (params (Key :type Key%20Structure :default "None"))
  (:Pressed
    (Character|Jump)))

(event Input|ActionEvents|InputActionSwitchCharacter
  (params (Key :type Key%20Structure :default "None"))
  (:Pressed
    (bind _outrownames (DataTable|GetDataTableRowNames "/Game/Pedestrians/CharacterTable.CharacterTable"))
    (bind _returnvalue (Utilities|GetDataTableRow "/Game/Pedestrians/CharacterTable.CharacterTable" (Utilities|Array|Get(acopy) _outrownames (Math|Random|RandomInteger (Variables|Default|GetmeshCount))))
      (:then
        (Class|SkinnedMeshComponent|SetSkeletalMesh (Variables|Character|GetMesh) (.charactermesh _returnvalue) false)))))

(event Input|ActionEvents|InputActionInteract
  (params (Key :type Key%20Structure :default "None"))
  (:Pressed
    (CallFunction|VehicleDetection)
    (Utilities|IsValid (Variables|Default|GetDetectedVehicle)
      (:Is%20Valid
        (CallFunction|PossesVehicle)))))

(event Input|AxisEvents|InputAxisThrottle
  (params (AxisValue :type Float%20%28single-precision%29))
  (Pawn|Input|AddMovementInput (Math|Vector|GetForwardVector (Math|Rotator|MakeRotator 0.0 0.0 (.yaw (Pawn|GetControlRotation :!class /Script/Engine.Pawn)))) AxisValue false))

(event Input|AxisEvents|InputAxisSteering
  (params (AxisValue :type Float%20%28single-precision%29))
  (Pawn|Input|AddMovementInput (Math|Vector|GetRightVector (Math|Rotator|MakeRotator 0.0 0.0 (.yaw (Pawn|GetControlRotation :!class /Script/Engine.Pawn)))) AxisValue false))

(event Input|AxisEvents|InputAxisCameraLook
  (params (AxisValue :type Float%20%28single-precision%29))
  (Pawn|Input|AddControllerYawInput AxisValue))

(fn ConstructionScript)

(fn VehicleDetection
  (bind _capsulecomponent (Variables|Collision|GetCapsuleComponent))
  (bind _returnvalue (Transformation|GetWorldLocation _capsulecomponent))
  (bind _outhit (Class|KismetSystemLibrary|BoxTraceSingleforObjects _returnvalue (+ _returnvalue (* (Math|Vector|GetForwardVector _capsulecomponent) 100)) "10.000000,10.000000,10.000000" "0, 0, 0" (Variables|Default|GetDetectableObjects) false 0 "None" true))
  (bind _asbp_controllable_vehicle (Utilities|Casting|CastToBP_ControllableVehicle (.hitactor _outhit))
    (:then
      (Utilities|IsValid _asbp_controllable_vehicle
        (:Is%20Valid
          (Variables|Default|SetDetectedVehicle _asbp_controllable_vehicle))))
    (:CastFailed
      (Variables|Default|SetDetectedVehicle 0))))

(fn RepossesfromVehicle
  (Transformation|DetachFromActor "KeepWorld" "KeepWorld" "KeepWorld")
  (Collision|SetActorEnableCollision self true)
  (Variables|Default|SetinVehicle false)
  (Pawn|Possess (Game|GetPlayerController 0) self))

(fn PossesVehicle
  (bind _self self)
  (bind _detectedvehicle (Variables|Default|GetDetectedVehicle))
  (Variables|Default|SetinVehicle true)
  (Collision|SetActorEnableCollision _self false)
  (Transformation|AttachActorToActor _self (Variables|Default|GetDetectedVehicle) "Driver" "SnapToTarget" "SnapToTarget" "SnapToTarget" true)
  (Variables|/Game/Vehicles/BP_ControllableVehicle.BP_ControllableVehicle_C|SetDriver _detectedvehicle self)
  (Pawn|Possess (Game|GetPlayerController 0) _detectedvehicle))